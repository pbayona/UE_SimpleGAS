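; Gameplay Ability for a base attack that commits, plays a dash montage, then an attack montage.
; A forward root motion constant force, with strength and duration at zero here, gates the switch between montages.
; During the attack, the first Event.Damage gameplay event sends a GE_DealDamage spec to the payload's target, passing Damage through SetByCaller.
; The ability ends when the attack montage completes, blends out or is stopped.
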(event `self.K2_ActivateAbility`
  (bind _returnvalue (`self.K2_CommitAbility`))
  (if _returnvalue
    (`AbilityTask_ApplyRootMotionConstantForce.ApplyRootMotionConstantForce` "None" (`Actor.GetActorForwardVector` (`self.GetAvatarActorFromActorInfo`)) 0.0 0.0 false "/Engine/Tutorial/ContentIntroCurve.ContentIntroCurve" "MaintainLastRootMotionVelocity"
      (:`then`
        (`AbilityTask_PlayMontageAndWait.CreatePlayMontageAndWaitProxy` "None" (`self.DashAnimation`)))
      (:`OnFinish`
        (`self.MontageStop` -1.0)
        (`AbilityTask_PlayMontageAndWait.CreatePlayMontageAndWaitProxy` "None" (`self.AttackAnimation`)
          (:`then`
            (bind (_asynctaskproxy _payload) (`AbilityTask_WaitGameplayEvent.WaitGameplayEvent` (struct :`TagName` "Event.Damage") null true)
              (:`EventReceived`
                (bind _result (`/Engine/EditorBlueprintResources/StandardMacros.NegateFloat` (`self.Damage`))
                  (:`  `
                    (bind _returnvalue_2 (`AbilitySystemBlueprintLibrary.AssignTagSetByCallerMagnitude` (`self.MakeOutgoingGameplayEffectSpec` "/Game/Gameplay/Effects/GE_DealDamage.GE_DealDamage_C") (struct :`TagName` "Event.Damage") _result))
                    (`AbilitySystemComponent.BP_ApplyGameplayEffectSpecToTarget` (`AbilitySystemBlueprintLibrary.GetAbilitySystemComponent` (`self.GetAvatarActorFromActorInfo`)) _returnvalue_2 (`AbilitySystemBlueprintLibrary.GetAbilitySystemComponent` (`.Target` (break `GameplayEventData` _payload)))))))))
          (:`OnCompleted`
            (`self.K2_EndAbility` :!label _label))
          (:`OnBlendOut`
            (goto _label))
          (:`OnInterrupted`
            (goto _label))
          (:`OnCancelled`
            (goto _label)))))
    (else
      (`self.K2_EndAbility`))))

(event `self.K2_OnEndAbility`
  (params (bWasCancelled :type Boolean))
  (`KismetSystemLibrary.PrintString` "Ability Performed"))